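; Player character for a 2D flying, auto-moving cat game with vertical input, lives, shield and timed levels.
; Tick applies the current displacement and tracks distance, checkpoints for respawns, level time and cat hunger, broadcasting stats through inform events.
; Obstacle and perk effects override displacement, with the shield absorbing obstacles.
; An unfed cat goes crazy, halting forward displacement for a few seconds; level-end and success widgets show distance as score.
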(event Custom|UpdateAnimation
  ;[1 1 1] animation change
  (Sprite|SetFlipbook (Variables|Default|GetSprite) "/Game/Flipbooks/crazyCat.crazyCat")
  (CallFunction|PerformMovementEffect "0, 0, 0" "NewEnumerator0" "NewEnumerator1")
  (Audio|Components|Audio|Play (Variables|Default|GetCatCrazy) 0.0)
  (Utilities|FlowControl|Delay 5.0)
  (CallFunction|RestoreMovementtoNormal)
  (Audio|Components|Audio|Stop (Variables|Default|GetCatCrazy)))

(event Custom|Event%20Update%20Distance
  ;[1 1 1] Distance
  (CallFunction|UpdateDistance))

(event Custom|Event%20Init%20Movement
  ;[1 1 1] movement
  (CallFunction|InitMovement))

(event Custom|Event%20Update%20Movement%20Mode
  ;[1 1 1] movement
  (CallFunction|Move (Variables|Default|GetcurrentDisplacement)))

(event Custom|Event%20Init%20Replication
  ;[1 1 1] replication
  (Class|ActorComponent|SetIsReplicated (Variables|Default|GetSprite) false))

(event Custom|Event%20Update%20Checkpoint
  ;[1 1 1] Distance
  (CallFunction|UpdateCheckPoint))

(event Custom|Event%20Update%20Duration
  ;[1 1 1] Duration
  (CallFunction|UpdateDuration)
  (CallFunction|UpdateCatHungerDuration))

(event EventBeginPlay
  (CallFunction|EventInitReplication)
  (CallFunction|EventInitMovement)
  (Sprite|SetFlipbook (Variables|Default|GetSprite) "/Game/Flipbooks/charIdle.charIdle"))

(event EventTick
  (params (DeltaSeconds :type Float%20%28single-precision%29))
  (CallFunction|EventUpdateMovementMode)
  (CallFunction|EventUpdateDistance)
  (CallFunction|EventUpdateCheckpoint)
  (CallFunction|EventUpdateDuration))

(event Input|AxisEvents|InputAxisMoveUp
  (params (AxisValue :type Float%20%28single-precision%29))
  ;[1 1 1] Player Controls
  (Pawn|Input|AddMovementInput "0.000000, 0,0.030000" AxisValue false))

(fn ConstructionScript)

(fn Move
  (params (amount :type Vector))
  (Pawn|Input|AddMovementInput amount (Utilities|Time|GetWorldDeltaSeconds) true))

(fn InitforLevel
  (params (maxDuration :type Float%20%28single-precision%29))
  (Variables|Default|Setlives 2)
  (Variables|Default|Setdistance 0)
  (CallFunction|UseShield)
  (Variables|Default|SetmaxDuration maxDuration)
  (Variables|Default|Setduration 0.0)
  (Variables|Default|SetcatHungerDuration 0.0)
  (Variables|Default|SetisCatCrazy false)
  (Variables|Default|SetisLevelEnded false)
  (CallFunction|CreateCharacterUI))

(fn UpdateDistance
  (bind _returnvalue (Transformation|GetActorLocation))
  (bind _x (Math|Vector|BreakVector _returnvalue))
  (bind _returnvalue_2 (/ _x 1e+02))
  (if (> _returnvalue_2 (Math|Conversions|ToFloat(Integer) (+ (Variables|Default|Getdistance) 1)))
    (bind _output_get (Variables|Default|Setdistance (Math|Float|Truncate _returnvalue_2)))
    (Default|CallEventInformDistance _output_get)))

(fn UpdateCheckPoint
  (if (> (Variables|Default|Getdistance) (+ (.distance (Variables|Default|GetlastCheckPoint)) 20))
    (Variables|Default|SetlastCheckPoint (Utilities|Struct|MakeCheckPointInfo (Variables|Default|Getdistance) (Transformation|GetActorLocation)))))

(fn Die
  (if (> (Variables|Default|Getlives) 1)
    (bind _result (Math|Integer|DecrementInt (Variables|Default|Getlives))
      (:%20%20
        (bind _output_get (Variables|Default|Setlives _result))
        (Variables|Default|SethasShield false)
        (CallFunction|StartfromLastCheckpoint)
        (Default|CallEventInformLives _output_get)))
    (else
      (CallFunction|EndLevel)
      (return true))))

(fn StartfromLastCheckpoint
  (bind _lastcheckpoint (Variables|Default|GetlastCheckPoint))
  (Variables|Default|Setdistance (.distance _lastcheckpoint))
  (Transformation|SetActorLocation (.position _lastcheckpoint) false true))

(fn EndLevel
  (bind _returnvalue (UserInterface|CreateWidget "/Game/Blueprints/LevelEndUI.LevelEndUI_C"))
  (Variables|/Game/Blueprints/LevelEndUI.LevelEndUI_C|Setscore _returnvalue (Variables|Default|Getdistance))
  (UserInterface|Viewport|AddtoViewport _returnvalue 0)
  (Variables|/Script/Engine.PlayerController|SetbShowMouseCursor (Game|GetPlayerController 0) true))

(fn InitDuration
  (Variables|Default|Setduration 0.0))

(fn UpdateDuration
  (bind _output_get (Variables|Default|Setduration (+ (Variables|Default|Getduration) (Utilities|Time|GetWorldDeltaSeconds))))
  (Utilities|FlowControl|Sequence
    (:then_0
      (Default|CallEventInformDuration (Variables|Default|Getduration)))
    (:then_1
      (if (and (>= _output_get (Variables|Default|GetmaxDuration)) (not (Variables|Default|GetisLevelEnded)))
        (Variables|Default|SetisLevelEnded true)
        (CallFunction|EndLevel)))))

(fn CreateCharacterUI
  (bind _returnvalue (UserInterface|CreateWidget "/Game/Blueprints/CharacterUI.CharacterUI_C" (.AsPlayer%20Controller (Utilities|Casting|CastToPlayerController (Pawn|GetController)))))
  (UserInterface|Viewport|AddtoViewport _returnvalue 0)
  (Default|CallEventInformDistance (Variables|Default|Getdistance))
  (Default|CallEventInformLives (Variables|Default|Getlives))
  (Default|CallEventInformDuration (Variables|Default|Getduration)))

(fn InitMovement
  (Variables|Default|SetcurrentDisplacement (Variables|Default|GetnormalDisplacement))
  (Variables|Default|SetcurrentMovementMode "NewEnumerator0")
  (Pawn|Components|CharacterMovement|SetMovementMode (Variables|Character|GetCharacterMovement) "MOVE_Flying" 0))

(fn PerformMovementEffect
  (params (displacement :type Vector) (movementMode :type MovementModes%20Enum) (type :type CollectableTypes%20Enum))
  (switch Utilities|FlowControl|Switch|SwitchonCollectableTypes type
    (:NewEnumerator0
      (if (Variables|Default|GethasShield)
        (CallFunction|UseShield)
        (return false)
        (else
          _)))
    (:NewEnumerator1
      _))
  (Variables|Default|SetcurrentDisplacement displacement)
  (Variables|Default|SetcurrentMovementMode movementMode)
  (return true))

(fn RestoreMovementtoNormal
  (Variables|Default|SetcurrentDisplacement (Variables|Default|GetnormalDisplacement))
  (Variables|Default|SetcurrentMovementMode "NewEnumerator0"))

(fn ActivateShield
  (bind _output_get (Variables|Default|SethasShield true))
  (Default|CallEventInformShield _output_get))

(fn UseShield
  (bind _output_get (Variables|Default|SethasShield false))
  (Default|CallEventInformShield _output_get)
  (return _output_get))

(fn IncrementLives
  (bind _result (Math|Integer|IncrementInt (Variables|Default|Getlives))
    (:%20%20
      (bind _output_get (Variables|Default|Setlives _result))
      (Default|CallEventInformLives _output_get))))

(fn DecreaseLives
  (bind _result (Math|Integer|DecrementInt (Variables|Default|Getlives))
    (:%20%20
      (Variables|Default|Setlives _result)
      (Utilities|FlowControl|Sequence
        (:then_0
          (Default|CallEventInformLives (Variables|Default|Getlives)))
        (:then_1
          (if (== (Variables|Default|Getlives) 0)
            (CallFunction|EndLevel)))))))

(fn ApplyPostProcessEffect
  (params (postProcess :type Post%20Process%20Component%20Object%20Reference)))

(fn UpdateCatHungerDuration
  (bind _output_get (Variables|Default|SetcatHungerDuration (+ (Variables|Default|GetcatHungerDuration) (Utilities|Time|GetWorldDeltaSeconds))))
  (Default|CallEventInformCatHungerDuration _output_get)
  (if (and (>= _output_get 35.0) (not (Variables|Default|GetisCatCrazy)))
    (Variables|Default|SetisCatCrazy true)
    (CallFunction|UpdateAnimation)))

(fn FeedCat
  (Variables|Default|SetisCatCrazy false)
  (Variables|Default|SetcatHungerDuration 0.0)
  (Sprite|SetFlipbook (Variables|Default|GetSprite) "/Game/Flipbooks/charIdle.charIdle"))

(fn Success
  (bind _returnvalue (UserInterface|CreateWidget "/Game/Blueprints/LevelSuccessUI.LevelSuccessUI_C"))
  (Variables|/Game/Blueprints/LevelSuccessUI.LevelSuccessUI_C|Setscore _returnvalue (Variables|Default|Getdistance))
  (UserInterface|Viewport|AddtoViewport _returnvalue 0)
  (Variables|/Script/Engine.PlayerController|SetbShowMouseCursor (Game|GetPlayerController 0) true))