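; CollectibleRain is a collectible that switches on a temporary post-process effect when picked up.
; It starts with PostProcess1 deactivated and disabled, and leaves overlap handling to its parent class first.
; If HasPerformed is then true, it activates and enables the component, waits for Duration, then calls Deactivate without clearing the Enabled flag.
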(event EventBeginPlay
  (bind _postprocess1 (Variables|Default|GetPostProcess1))
  (Components|Activation|Deactivate _postprocess1)
  (Variables|/Script/Engine.PostProcessComponent|SetbEnabled _postprocess1 false))

(event Collision|EventActorBeginOverlap
  (params (OtherActor :type Actor%20Object%20Reference))
  (bind _postprocess1 (Variables|Default|GetPostProcess1))
  (|CallParentFunction OtherActor)
  (if (Variables|Default|GethasPerformed)
    (Components|Activation|Activate _postprocess1 false)
    (Variables|/Script/Engine.PostProcessComponent|SetbEnabled _postprocess1 true)
    (Utilities|FlowControl|Delay (Variables|Default|Getduration))
    (Components|Activation|Deactivate _postprocess1)))

(fn ConstructionScript
  (|CallParentFunction))