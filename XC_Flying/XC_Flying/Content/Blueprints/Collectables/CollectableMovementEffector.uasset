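; CollectableMovementEffector is a pickup that temporarily alters the movement of the player character that overlaps it.
; On overlap with a MyCharacter it hides itself, disables collision and passes its Displacement and MovementMode to the character's PerformMovementEffect.
; The actor stays alive through a Duration delay to time the effect, then calls RestoreMovementToNormal on the stored player and destroys itself.
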(event Collision|EventActorBeginOverlap
  (params (OtherActor :type Actor%20Object%20Reference))
  (bind _asmy_character (Utilities|Casting|CastToMyCharacter OtherActor))
  (Rendering|SetVisibility (Variables|Default|GetDefaultSceneRoot) false true)
  (Collision|SetActorEnableCollision false)
  (bind _output_get (Variables|Default|SetoverlappingPlayer _asmy_character))
  (Default|PerformMovementEffect _output_get (Variables|Default|Getdisplacement) (Variables|Default|GetmovementMode) "NewEnumerator0")
  (Utilities|FlowControl|Delay (Variables|Default|Getduration))
  (Default|RestoreMovementtoNormal (Variables|Default|GetoverlappingPlayer))
  (CallFunction|Destroy))

(fn ConstructionScript
  (|CallParentFunction))