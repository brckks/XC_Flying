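; CollectableSun is a collectable actor that applies a temporary post-process effect when picked up.
; Its PostProcess component starts deactivated and disabled at BeginPlay.
; On overlap it runs the parent's handling, then, if HasPerformed is set, activates and enables the effect.
; After Duration it calls Deactivate but leaves the Enabled flag true.
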(event EventBeginPlay
  (bind _postprocess (Variables|Default|GetPostProcess))
  (Components|Activation|Deactivate _postprocess)
  (Variables|/Script/Engine.PostProcessComponent|SetbEnabled _postprocess false))

(event Collision|EventActorBeginOverlap
  (params (OtherActor :type Actor%20Object%20Reference))
  (bind _postprocess (Variables|Default|GetPostProcess))
  (|CallParentFunction OtherActor)
  (if (Variables|Default|GethasPerformed)
    (Components|Activation|Activate _postprocess false)
    (Variables|/Script/Engine.PostProcessComponent|SetbEnabled _postprocess true)
    (Utilities|FlowControl|Delay (Variables|Default|Getduration))
    (Components|Activation|Deactivate _postprocess)))

(event EventTick
  (params (DeltaSeconds :type Float%20%28single-precision%29)))

(fn ConstructionScript
  (|CallParentFunction))