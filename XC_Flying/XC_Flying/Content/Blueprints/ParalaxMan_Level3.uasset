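; Parallax background manager for Level 3 that scrolls three sprite layers as the player moves.
; On BeginPlay it caches the player pawn as MyCharacter.
; Each Tick, UpdateBackground shifts each sprite along world X by its layer speed times the X of the player's last movement input vector.
; The shift follows input rather than actual velocity and is not scaled by delta time, so scroll speed depends on frame rate.
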(event EventBeginPlay
  (bind _asmy_character (Utilities|Casting|CastToMyCharacter (Game|Player|GetPlayerPawn 0)))
  (Variables|Default|Setplayer _asmy_character))

(event Collision|EventActorBeginOverlap
  (params (OtherActor :type Actor%20Object%20Reference)))

(event EventTick
  (params (DeltaSeconds :type Float%20%28single-precision%29))
  (CallFunction|UpdateBackground (Variables|Default|Getlon2_Sprite) (Variables|Default|Getbg2Speed))
  (CallFunction|UpdateBackground (Variables|Default|Getlon3_Sprite) (Variables|Default|Getbg3Speed))
  (CallFunction|UpdateBackground (Variables|Default|Getlon4_Sprite) (Variables|Default|Getbg4Speed)))

(fn ConstructionScript)

(fn UpdateBackground
  (params (bg :type Paper%20Sprite%20Component%20Object%20Reference) (speed :type Float%20%28single-precision%29))
  (bind _returnvalue (Transformation|GetWorldLocation bg))
  (Transformation|SetWorldLocation bg (Math|Vector|MakeVector (+ (.x _returnvalue) (* speed (.x (Class|Pawn|GetLastMovementInputVector (Variables|Default|Getplayer))))) (.y _returnvalue) (.z _returnvalue)) false false)
  (return))