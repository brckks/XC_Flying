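; Parallax manager actor that scrolls three background layers horizontally in response to player movement.
; BeginPlay caches the player pawn as MyCharacter.
; Each Tick, UpdateBgMovement shifts Bg2, Bg3 and Bg4 along world X by their own speed times the player's last movement input X.
; The offset follows input rather than actual displacement and is not scaled by delta time, so scroll rate depends on frame rate.
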(event EventBeginPlay
  (bind _asmy_character (Utilities|Casting|CastToMyCharacter (Game|Player|GetPlayerPawn 0)))
  (Variables|Default|Setplayer _asmy_character))

(event Collision|EventActorBeginOverlap
  (params (OtherActor :type Actor%20Object%20Reference)))

(event EventTick
  (params (DeltaSeconds :type Float%20%28single-precision%29))
  (CallFunction|UpdateBgMovement (Variables|Default|Getbg3) (Variables|Default|GetbgThreeSpeed))
  (CallFunction|UpdateBgMovement (Variables|Default|Getbg2) (Variables|Default|GetbgTwoSpeed))
  (CallFunction|UpdateBgMovement (Variables|Default|Getbg4) (Variables|Default|GetbgFourSpeed)))

(fn ConstructionScript)

(fn UpdateBgMovement
  (params (bg :type Paper%20Sprite%20Component%20Object%20Reference) (speed :type Float%20%28single-precision%29))
  (bind _returnvalue (Transformation|GetWorldLocation bg))
  (Transformation|SetWorldLocation bg (Math|Vector|MakeVector (+ (.x _returnvalue) (* speed (.x (Class|Pawn|GetLastMovementInputVector (Variables|Default|Getplayer))))) (.y _returnvalue) (.z _returnvalue)) false false)
  (return))